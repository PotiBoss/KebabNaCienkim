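; BP_MainCharacterHead is an interactable main character head that the player can pick up.
; Its Interact override checks that BP_MainCharacter holds no valid PickedUpActor, then registers itself in that slot.
; It snaps onto the PickupSocket of the character's Sprite and calls the parent Interact only on a successful pickup.
; The event graph holds only disabled stub events.
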(event EventBeginPlay
  (|CallParentFunction) ; This node is disabled and will not be called.\nDrag off pins to build functionality.
)

(event Collision|EventActorBeginOverlap
  (params (OtherActor :type Actor%20Object%20Reference))
  (|CallParentFunction OtherActor) ; This node is disabled and will not be called.\nDrag off pins to build functionality.
)

(event EventTick
  (params (DeltaSeconds :type Float%20%28single-precision%29))
  (|CallParentFunction DeltaSeconds) ; This node is disabled and will not be called.\nDrag off pins to build functionality.
)

(fn ConstructionScript
  (|CallParentFunction))

(fn Interact
  (bind _asbp_main_character (Utilities|Casting|CastToBP_MainCharacter (Game|Player|GetPlayerPawn 0)))
  (Utilities|IsValid (Variables|/Game/KebabNaCienkim/Blueprint/Character/BP_MainCharacter.BP_MainCharacter_C|GetPickedUpActor _asbp_main_character)
    (:Is%20Not%20Valid
      (Variables|/Game/KebabNaCienkim/Blueprint/Character/BP_MainCharacter.BP_MainCharacter_C|SetPickedUpActor _asbp_main_character self)
      (Transformation|AttachComponentToComponent (Variables|/Script/Paper2D.PaperCharacter|GetSprite _asbp_main_character) "PickupSocket" "SnapToTarget" "SnapToTarget" "SnapToTarget" true)
      (|CallParentFunction))))