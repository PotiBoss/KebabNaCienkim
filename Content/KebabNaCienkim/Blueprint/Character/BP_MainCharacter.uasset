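; BP_MainCharacter is the player's 2D flipbook character, handling movement, interaction and the notes book.
; BeginPlay creates the book and dialog widgets; the Book input toggles the book and mouse cursor when notes are allowed.
; Axis inputs move it along world X and Z, gated by a book-visibility check, while Action calls Interact on the current interactable.
; Tick picks a directional walk or idle flipbook from velocity and last input direction.
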(event EventBeginPlay
  (bind _returnvalue (Game|GetPlayerController 0))
  ;[1 1 1] Creating book widget for pickups
  (bind _returnvalue_2 (UserInterface|CreateWidget "/Game/KebabNaCienkim/Blueprint/Notes/WBP_Book.WBP_Book_C" _returnvalue))
  (bind _output_get (Variables|Default|SetBookWidget _returnvalue_2))
  (Default|InitWidget _output_get self)
  (bind _returnvalue_3 (UserInterface|CreateWidget "/Game/KebabNaCienkim/Blueprint/Dialog/WBP_Dialog.WBP_Dialog_C" _returnvalue))
  (Variables|Default|SetDialogWidget _returnvalue_3))

(event EventTick
  (params (DeltaSeconds :type Float%20%28single-precision%29))
  (CallFunction|SetMyFlipBook))

(event Input|ActionEvents|InputActionBook
  (params (Key :type Key%20Structure :default "None"))
  (bind _bookwidget (Variables|Default|GetBookWidget))
  (:Pressed
    (if (Variables|Default|GetbCanOpenNotes)
      (Utilities|FlowControl|FlipFlop
        (:A
          (UserInterface|Viewport|AddtoViewport _bookwidget 0)
          (Variables|/Script/Engine.PlayerController|SetbShowMouseCursor (Game|GetPlayerController 0) true)
          (Default|WidgetOpen _bookwidget))
        (:B
          (Widget|RemovefromParent (Variables|Default|GetBookWidget))
          (Variables|/Script/Engine.PlayerController|SetbShowMouseCursor (Game|GetPlayerController 0) false))))))

(event Input|ActionEvents|InputActionAction
  (params (Key :type Key%20Structure :default "None"))
  (:Pressed
    (Utilities|IsValid (Variables|Default|GetInteractableActor)
      (:Is%20Valid
        (Default|Interact (Variables|Default|GetInteractableActor))))))

(event Input|AxisEvents|InputAxisMoveForward
  (params (AxisValue :type Float%20%28single-precision%29))
  (Utilities|MovementCheck
    (:false
      (Pawn|Input|AddMovementInput "0, 0,1.000000" AxisValue false))))

(event Input|AxisEvents|InputAxisMoveRight
  (params (AxisValue :type Float%20%28single-precision%29))
  (Utilities|MovementCheck
    (:false
      (Pawn|Input|AddMovementInput "1.000000, 0, 0" AxisValue false))))

(fn ConstructionScript)

(fn SetMyFlipBook
  (if (or (!= (Input|AxisValues|GetMoveForward) 0.0) (!= (Input|AxisValues|GetMoveRight) 0.0))
    (Variables|Default|SetLastMoveDirection (select (> (Input|AxisValues|GetMoveForward) 0.0) "NewEnumerator0" (select (< (Input|AxisValues|GetMoveForward) 0.0) "NewEnumerator1" (select (> (Input|AxisValues|GetMoveRight) 0.0) "NewEnumerator3" "NewEnumerator2")))))
  (Sprite|SetFlipbook (Variables|Default|GetSprite) (select (> (Math|Vector|VectorLength (Transformation|GetVelocity)) 0.0) (Utilities|Select :Index (Variables|Default|GetLastMoveDirection) :NewEnumerator0 "/Game/KebabNaCienkim/Blueprint/Character/Movement_Up.Movement_Up" :NewEnumerator1 "/Game/KebabNaCienkim/Blueprint/Character/Movement_Down.Movement_Down" :NewEnumerator2 "/Game/KebabNaCienkim/Blueprint/Character/Movement_Left.Movement_Left" :NewEnumerator3 "/Game/KebabNaCienkim/Blueprint/Character/Movement_Right.Movement_Right") (Utilities|Select :Index (Variables|Default|GetLastMoveDirection) :NewEnumerator0 "/Game/KebabNaCienkim/Blueprint/Character/Idle_Up.Idle_Up" :NewEnumerator1 "/Game/KebabNaCienkim/Blueprint/Character/Idle_Down.Idle_Down" :NewEnumerator2 "/Game/KebabNaCienkim/Blueprint/Character/Idle_Left.Idle_Left" :NewEnumerator3 "/Game/KebabNaCienkim/Blueprint/Character/Idle_Right.Idle_Right"))))