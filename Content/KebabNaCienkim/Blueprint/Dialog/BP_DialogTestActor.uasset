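; BP_DialogTestActor is an interactable test actor that starts a dialog with the player.
; On Interact it copies the table from its DialogComponent into the DialogWidget of BP_MainCharacter, calls StartDialog, then calls the parent Interact.
; An older, disconnected chain that added the widget to the viewport and fed it table rows by index remains but never runs.
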(event EventBeginPlay
  (|CallParentFunction) ; This node is disabled and will not be called.\nDrag off pins to build functionality.
)

(event Collision|EventActorBeginOverlap
  (params (OtherActor :type Actor%20Object%20Reference))
  (|CallParentFunction OtherActor) ; This node is disabled and will not be called.\nDrag off pins to build functionality.
)

(event EventTick
  (params (DeltaSeconds :type Float%20%28single-precision%29))
  (|CallParentFunction DeltaSeconds) ; This node is disabled and will not be called.\nDrag off pins to build functionality.
)

(fn ConstructionScript
  (|CallParentFunction))

(fn Interact
  (bind _asbp_main_character (Utilities|Casting|CastToBP_MainCharacter (Game|Player|GetPlayerPawn 0)))
  (Variables|/Game/KebabNaCienkim/Blueprint/Dialog/WBP_Dialog.WBP_Dialog_C|SetDialogTable (Variables|/Game/KebabNaCienkim/Blueprint/Character/BP_MainCharacter.BP_MainCharacter_C|GetDialogWidget _asbp_main_character) (Variables|/Game/KebabNaCienkim/Blueprint/Dialog/BP_DialogComponent.BP_DialogComponent_C|GetDialog%20Table (Variables|Default|GetDialogComponent)))
  (Default|StartDialog (Variables|/Game/KebabNaCienkim/Blueprint/Character/BP_MainCharacter.BP_MainCharacter_C|GetDialogWidget _asbp_main_character))
  (|CallParentFunction))