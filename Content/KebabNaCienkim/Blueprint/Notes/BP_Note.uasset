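; BP_Note is a collectible note that the player picks up by interacting with it.
; Interact enables note opening on the main character and marks the NotesArray entry at NoteIndex as collected.
; The same index reveals the matching button in the character's book widget.
; The actor then destroys itself and calls the parent Interact.
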(event EventBeginPlay)

(event Collision|EventActorBeginOverlap
  (params (OtherActor :type Actor%20Object%20Reference)))

(event EventTick
  (params (DeltaSeconds :type Float%20%28single-precision%29)))

(fn ConstructionScript)

(fn Interact
  (bind _maincharacter (Variables|Default|GetMainCharacter))
  (Variables|/Game/KebabNaCienkim/Blueprint/Character/BP_MainCharacter.BP_MainCharacter_C|SetbCanOpenNotes _maincharacter true)
  (Utilities|Struct|SetmembersinNotes (Utilities|Array|Get(acopy) (Variables|/Game/KebabNaCienkim/Blueprint/Character/BP_MainCharacter.BP_MainCharacter_C|GetNotesArray _maincharacter) (Variables|Default|GetNoteIndex)) true)
  (Widget|SetVisibility (Utilities|Array|Get(acopy) (Variables|/Game/KebabNaCienkim/Blueprint/Notes/WBP_Book.WBP_Book_C|GetButtonArray (Variables|/Game/KebabNaCienkim/Blueprint/Character/BP_MainCharacter.BP_MainCharacter_C|GetBookWidget _maincharacter)) (Variables|Default|GetNoteIndex)) "Visible")
  (Actor|DestroyActor)
  (|CallParentFunction))