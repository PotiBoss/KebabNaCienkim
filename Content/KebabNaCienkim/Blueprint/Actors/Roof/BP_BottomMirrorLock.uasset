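; BP_BottomMirrorLock is a roof quest trigger that locks the back mirror into place when it overlaps the collision component.
; On overlap with a BP_BackMirror it stops that mirror's physics and flags it as placed.
; It then finds the BP_FrontMirror and, if both mirrors are placed, enables the roof TP and switches the roof ghost to its post-quest dialog table.
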(event OnComponentBeginOverlap(CollisionComponent)
  (params (OverlappedComponent :type Primitive%20Component%20Object%20Reference) (OtherActor :type Actor%20Object%20Reference) (OtherComp :type Primitive%20Component%20Object%20Reference) (OtherBodyIndex :type Integer) (bFromSweep :type Boolean) (SweepResult :type Hit%20Result%20Structure%20%28by%20ref%29))
  (bind _asbp_back_mirror (Utilities|Casting|CastToBP_BackMirror OtherActor))
  (Physics|SetSimulatePhysics (Variables|/Script/Paper2D.PaperSpriteActor|GetRenderComponent _asbp_back_mirror) false)
  (bind _output_get (Variables|/Game/KebabNaCienkim/Blueprint/Actors/Roof/BP_BackMirror.BP_BackMirror_C|SetBackMirrorInPlaced? _asbp_back_mirror true))
  (bind _returnvalue (Actor|GetActorOfClass "/Game/KebabNaCienkim/Blueprint/Actors/Roof/BP_FrontMirror.BP_FrontMirror_C"))
  (if (and _output_get (Variables|/Game/KebabNaCienkim/Blueprint/Actors/Roof/BP_FrontMirror.BP_FrontMirror_C|GetFrontMirrorInPlaced? _returnvalue))
    (Variables|/Game/KebabNaCienkim/Blueprint/Actors/BP_TeleportIn.BP_TeleportIn_C|SetbIsEnabled? (Variables|Default|GetRoofTP) true)
    ;[1 0.0831 0.103] Here is where roof quest ends I guess?
    (Variables|/Game/KebabNaCienkim/Blueprint/Dialog/BP_DialogComponent.BP_DialogComponent_C|SetDialog%20Table (Variables|/Game/KebabNaCienkim/Blueprint/Actors/Roof/BP_RoofGhost.BP_RoofGhost_C|GetDialogComponent (Variables|Default|GetRoofGhost)) (Variables|Default|GetPostQuestDialog))))

(event EventBeginPlay)

(event Collision|EventActorBeginOverlap
  (params (OtherActor :type Actor%20Object%20Reference)))

(event EventTick
  (params (DeltaSeconds :type Float%20%28single-precision%29)))

(fn ConstructionScript)