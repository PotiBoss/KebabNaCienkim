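; BP_KitchenGhost is an interactable ghost that wants a specific food delivered by the player.
; On BeginPlay it picks one of the first two DT_Food rows at random for its sprite and FoodIndex.
; Interact compares this index with the player's carried BP_Food, which is destroyed either way.
; A match destroys the ghost and decrements Cook's GhostNumber, calling GhostsDestroyed on Cook when none remain.
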(event EventBeginPlay
  (bind _outrownames (DataTable|GetDataTableRowNames "/Game/KebabNaCienkim/Blueprint/Dialog/DT_Food.DT_Food"))
  (bind _returnvalue (Utilities|GetDataTableRow "/Game/KebabNaCienkim/Blueprint/Dialog/DT_Food.DT_Food" (Utilities|Array|Get(acopy) _outrownames (Math|Random|RandomInteger 2)))
    (:then
      (Rendering|Components|Sprite|SetSprite (Variables|Default|GetFoodSprite) (.sprite _returnvalue))
      (Variables|Default|SetFoodIndex (.index _returnvalue))
      (|CallParentFunction))))

(event Collision|EventActorBeginOverlap
  (params (OtherActor :type Actor%20Object%20Reference))
  (|CallParentFunction OtherActor) ; This node is disabled and will not be called.\nDrag off pins to build functionality.
)

(event EventTick
  (params (DeltaSeconds :type Float%20%28single-precision%29))
  (|CallParentFunction DeltaSeconds) ; This node is disabled and will not be called.\nDrag off pins to build functionality.
)

(fn ConstructionScript
  (|CallParentFunction))

(fn Interact
  (bind _cook (Variables|Default|GetCook))
  (bind _asbp_main_character (Utilities|Casting|CastToBP_MainCharacter (Game|Player|GetPlayerPawn 0)))
  (bind _asbp_food (Utilities|Casting|CastToBP_Food (Variables|/Game/KebabNaCienkim/Blueprint/Character/BP_MainCharacter.BP_MainCharacter_C|GetPickedUpActor _asbp_main_character)))
  (if (== (Variables|Default|GetFoodIndex) (Variables|/Game/KebabNaCienkim/Blueprint/Actors/BP_Food.BP_Food_C|GetFoodIndex _asbp_food))
    (bind _output_get (Variables|/Game/KebabNaCienkim/Blueprint/Actors/BP_Cook.BP_Cook_C|SetGhostNumber _cook (- (Variables|/Game/KebabNaCienkim/Blueprint/Actors/BP_Cook.BP_Cook_C|GetGhostNumber _cook) 1)))
    (if (< _output_get 1)
      (Default|GhostsDestroyed (Variables|Default|GetCook)))
    (Actor|DestroyActor))
  (Actor|DestroyActor _asbp_food)
  (|CallParentFunction))