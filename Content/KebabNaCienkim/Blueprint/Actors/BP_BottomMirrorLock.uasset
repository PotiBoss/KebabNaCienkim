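; BP_BottomMirrorLock is a trigger actor that locks the back mirror in place as part of completing the roof level.
; When its collision component overlaps a BP_BackMirror, it turns off the mirror's physics simulation and flags it as placed.
; It then finds the BP_FrontMirror in the level and, if that is also placed, calls RoofLevelCompleted on BP_MainGameMode.
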(event OnComponentBeginOverlap(CollisionComponent)
  (params (OverlappedComponent :type Primitive%20Component%20Object%20Reference) (OtherActor :type Actor%20Object%20Reference) (OtherComp :type Primitive%20Component%20Object%20Reference) (OtherBodyIndex :type Integer) (bFromSweep :type Boolean) (SweepResult :type Hit%20Result%20Structure%20%28by%20ref%29))
  (bind _asbp_back_mirror (Utilities|Casting|CastToBP_BackMirror OtherActor))
  (Physics|SetSimulatePhysics (Variables|/Script/Paper2D.PaperSpriteActor|GetRenderComponent _asbp_back_mirror) false)
  (bind _output_get (Variables|/Game/KebabNaCienkim/Blueprint/Actors/BP_BackMirror.BP_BackMirror_C|SetBackMirrorInPlaced? _asbp_back_mirror true))
  (bind _returnvalue (Actor|GetActorOfClass "/Game/KebabNaCienkim/Blueprint/Actors/BP_FrontMirror.BP_FrontMirror_C"))
  (if (and _output_get (Variables|/Game/KebabNaCienkim/Blueprint/Actors/BP_FrontMirror.BP_FrontMirror_C|GetFrontMirrorInPlaced? _returnvalue))
    (bind _asbp_main_game_mode (Utilities|Casting|CastToBP_MainGameMode (Game|GetGameMode)))
    (Default|RoofLevelCompleted _asbp_main_game_mode)))

(event EventBeginPlay)

(event Collision|EventActorBeginOverlap
  (params (OtherActor :type Actor%20Object%20Reference)))

(event EventTick
  (params (DeltaSeconds :type Float%20%28single-precision%29)))

(fn ConstructionScript)