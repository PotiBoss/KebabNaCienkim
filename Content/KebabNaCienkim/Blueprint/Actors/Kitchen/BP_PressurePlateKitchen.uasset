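; BP_PressurePlateKitchen is an interactable kitchen plate that spawns food while a player's detachable head rests on it.
; Interacting with a carried BP_MainCharacterHead drops it onto the plate, then spawns a BP_Food above and calls the parent Interact.
; Interacting again destroys the food, calls the head's Interact and re-registers the plate as the player's interactable.
; Ending capsule overlap also destroys the food when no head is present.
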(event OnComponentEndOverlap(Capsule)
  (params (OverlappedComponent :type Primitive%20Component%20Object%20Reference) (OtherActor :type Actor%20Object%20Reference) (OtherComp :type Primitive%20Component%20Object%20Reference) (OtherBodyIndex :type Integer))
  (bind _food (Variables|Default|GetFood))
  (Utilities|IsValid _food
    (:Is%20Valid
      (if (not (Variables|Default|GetbHasHead))
        (Actor|DestroyActor _food)))))

(event EventBeginPlay
  (|CallParentFunction) ; This node is disabled and will not be called.\nDrag off pins to build functionality.
)

(event Collision|EventActorBeginOverlap
  (params (OtherActor :type Actor%20Object%20Reference))
  (|CallParentFunction OtherActor) ; This node is disabled and will not be called.\nDrag off pins to build functionality.
)

(event EventTick
  (params (DeltaSeconds :type Float%20%28single-precision%29))
  (|CallParentFunction DeltaSeconds) ; This node is disabled and will not be called.\nDrag off pins to build functionality.
)

(fn ConstructionScript
  (|CallParentFunction))

(fn Interact
  (bind _food (Variables|Default|GetFood))
  (Utilities|IsValid _food
    (:Is%20Valid
      (Actor|DestroyActor _food))
    (:Is%20Not%20Valid
      _))
  (if (Variables|Default|GetbHasHead)
    (CallFunction|Interact (Variables|Default|GetHead))
    (Variables|Default|SetbHasHead false)
    (bind _asbp_main_character (Utilities|Casting|CastToBP_MainCharacter (Game|Player|GetPlayerPawn 0)))
    (Variables|/Game/KebabNaCienkim/Blueprint/Character/BP_MainCharacter.BP_MainCharacter_C|SetInteractableActor _asbp_main_character self)
    (else
      (bind _asbp_main_character_2 (Utilities|Casting|CastToBP_MainCharacter (Game|Player|GetPlayerPawn 0)))
      (bind _asbp_main_character_head (Utilities|Casting|CastToBP_MainCharacterHead (Variables|/Game/KebabNaCienkim/Blueprint/Character/BP_MainCharacter.BP_MainCharacter_C|GetPickedUpActor _asbp_main_character_2)))
      (Default|DropPickup _asbp_main_character_2)
      (Transformation|SetActorLocation _asbp_main_character_head (Transformation|GetActorLocation) false false)
      (Variables|Default|SetbHasHead true)
      (Variables|Default|SetHead _asbp_main_character_head)
      (CallFunction|SpawnNewFood)
      (|CallParentFunction))))

(fn SpawnNewFood
  (bind _returnvalue (Transformation|GetActorTransform))
  (bind _returnvalue_2 (Game|SpawnActorfromClass "/Game/KebabNaCienkim/Blueprint/Actors/Kitchen/BP_Food.BP_Food_C" (Math|Transform|MakeTransform (Math|Vector|MakeVector (.x (.location _returnvalue)) (.y (.location _returnvalue)) (+ (.z (.location _returnvalue)) 2.3e+02)) (.rotation _returnvalue) (.scale _returnvalue)) "Undefined" 0 0))
  (bind _output_get (Variables|Default|SetFood _returnvalue_2))
  (Default|Spawn _output_get))