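; BP_Hedge is a garden hedge sprite actor that the player can crop with pruning scissors.
; Its box overlap enables input for BP_MainCharacter while the hedge is uncropped and disables it on exit.
; Pressing E with the scissors picked up marks it cropped, notifies CounterRef and disables input.
; Tick swaps between cropped and uncropped sprites every frame, with the render component set to Movable at BeginPlay.
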(event OnComponentBeginOverlap(Box)
  (params (OverlappedComponent :type Primitive%20Component%20Object%20Reference) (OtherActor :type Actor%20Object%20Reference) (OtherComp :type Primitive%20Component%20Object%20Reference) (OtherBodyIndex :type Integer) (bFromSweep :type Boolean) (SweepResult :type Hit%20Result%20Structure%20%28by%20ref%29))
  ;[1 1 1] Disable/Enable input around the Hedge
  (Utilities|Casting|CastToBP_MainCharacter OtherActor)
  (if (not (Variables|Default|GetbIsCropped))
    (Input|EnableInput (Game|GetPlayerController 0))))

(event OnComponentEndOverlap(Box)
  (params (OverlappedComponent :type Primitive%20Component%20Object%20Reference) (OtherActor :type Actor%20Object%20Reference) (OtherComp :type Primitive%20Component%20Object%20Reference) (OtherBodyIndex :type Integer))
  ;[1 1 1] Disable/Enable input around the Hedge
  (Utilities|Casting|CastToBP_MainCharacter OtherActor)
  (Input|DisableInput (Game|GetPlayerController 0)))

(event EventTick
  (params (DeltaSeconds :type Float%20%28single-precision%29))
  ;[1 1 1] Change the sprite on the object whether is it cropped or not
  (if (Variables|Default|GetbIsCropped)
    (Rendering|Components|Sprite|SetSprite (Variables|Default|GetRenderComponent) (Variables|Default|GetCroppedSprite))
    (else
      (Rendering|Components|Sprite|SetSprite (Variables|Default|GetRenderComponent) (Variables|Default|GetUncroppedSprite)))))

(event EventBeginPlay
  ;[1 1 1] Set the mobility to movable to be albe to change the sprite on the object
  (Transformation|SetMobility (Variables|Default|GetRenderComponent) "Movable")
  (Physics|SetEnableGravity (Variables|Default|GetRenderComponent) false))

(event Input|KeyboardEvents|E
  (params (Key :type Key%20Structure :default "None"))
  ;[1 1 1] E event responsible for setting the IsCropped bool and call counter functions
  (:Pressed
    (if (Variables|/Game/KebabNaCienkim/Blueprint/Actors/Garden/BP_PruningScissors.BP_PruningScissors_C|GetbIsPickedUp (Variables|Default|GetPruningScissors))
      (bind _output_get (Variables|Default|SetbIsCropped true))
      (Default|CroppedCounter (Variables|Default|GetCounterRef) _output_get)
      (Input|DisableInput (Game|GetPlayerController 0)))))

(fn ConstructionScript)