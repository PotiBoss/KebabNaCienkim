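; BP_CountCroppedHedges is a garden actor that tracks how many hedges are cropped and notifies the Gardener at a target total.
; CroppedCounter raises or lowers the count based on its IsCropped flag, then calls HedgeDestroyed on the Gardener when the count equals twelve.
; The event graph holds only disabled stubs, and a disconnected node that would enable TPRef never runs.
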(event EventBeginPlay)

(event Collision|EventActorBeginOverlap
  (params (OtherActor :type Actor%20Object%20Reference)))

(event EventTick
  (params (DeltaSeconds :type Float%20%28single-precision%29)))

(fn ConstructionScript)

(fn CroppedCounter
  (params (IsCropped :type Boolean))
  (if IsCropped
    (Variables|Default|SetCroppedHedges (+ (Variables|Default|GetCroppedHedges) 1))
    (else
      (Variables|Default|SetCroppedHedges (+ (Variables|Default|GetCroppedHedges) -1))))
  (if (== (Variables|Default|GetCroppedHedges) 12)
    (Default|HedgeDestroyed (Variables|Default|GetGardener))))