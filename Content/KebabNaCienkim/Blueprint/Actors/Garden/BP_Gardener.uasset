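; BP_Gardener is the gardener, an interactable actor that holds dialog and reacts to the destruction of a hedge.
; Interacting runs its DialogComponent, then passes the call on to the parent implementation.
; HedgeDestroyed swaps the dialog table to a post-hedge one and enables a referenced Teleport.
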(event EventBeginPlay
  (|CallParentFunction))

(event Collision|EventActorBeginOverlap
  (params (OtherActor :type Actor%20Object%20Reference))
  (|CallParentFunction OtherActor) ; This node is disabled and will not be called.\nDrag off pins to build functionality.
)

(event EventTick
  (params (DeltaSeconds :type Float%20%28single-precision%29))
  (|CallParentFunction DeltaSeconds) ; This node is disabled and will not be called.\nDrag off pins to build functionality.
)

(fn ConstructionScript
  (|CallParentFunction))

(fn Interact
  (Default|DialogInteract (Variables|Default|GetDialogComponent))
  (|CallParentFunction))

(fn HedgeDestroyed
  (Variables|/Game/KebabNaCienkim/Blueprint/Dialog/BP_DialogComponent.BP_DialogComponent_C|SetDialog%20Table (Variables|Default|GetDialogComponent) (Variables|Default|GetPostHedgeTable))
  (Variables|/Game/KebabNaCienkim/Blueprint/Actors/BP_TeleportIn.BP_TeleportIn_C|SetbIsEnabled? (Variables|Default|GetTeleport) true))