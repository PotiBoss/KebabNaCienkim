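; BP_TeleportIn is the entry point of a teleporter that sends the player character to a linked TPOut.
; Overlapping its EnableDisableInput component enables input on the actor for BP_MainCharacter, and leaving disables it.
; Pressing E while IsEnabled is true teleports the player to TPOut's stored transform location, then clears IsEnabled, which nothing in this graph restores.
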(event OnComponentBeginOverlap(EnableDisableInput)
  (params (OverlappedComponent :type Primitive%20Component%20Object%20Reference) (OtherActor :type Actor%20Object%20Reference) (OtherComp :type Primitive%20Component%20Object%20Reference) (OtherBodyIndex :type Integer) (bFromSweep :type Boolean) (SweepResult :type Hit%20Result%20Structure%20%28by%20ref%29))
  (Utilities|Casting|CastToBP_MainCharacter OtherActor)
  (Input|EnableInput (Game|GetPlayerController 0)))

(event OnComponentEndOverlap(EnableDisableInput)
  (params (OverlappedComponent :type Primitive%20Component%20Object%20Reference) (OtherActor :type Actor%20Object%20Reference) (OtherComp :type Primitive%20Component%20Object%20Reference) (OtherBodyIndex :type Integer))
  (Utilities|Casting|CastToBP_MainCharacter OtherActor)
  (Input|DisableInput (Game|GetPlayerController 0)))

(event Input|KeyboardEvents|E
  (params (Key :type Key%20Structure))
  (:Pressed
    (if (Variables|Default|GetbIsEnabled?)
      (Transformation|SetActorTransform (Game|GetPlayerCharacter 0) (Math|Transform|MakeTransform (.location (Variables|/Game/KebabNaCienkim/Blueprint/Actors/BP_TeleportOut.BP_TeleportOut_C|GetTPOutTransform (Variables|Default|GetTPOut))) "0, 0, 0" "1.000000,1.000000,1.000000") false true)
      (Variables|Default|SetbIsEnabled? false))))

(fn ConstructionScript)